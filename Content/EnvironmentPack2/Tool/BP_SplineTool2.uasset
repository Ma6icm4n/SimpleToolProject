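; BP_SplineTool2 is an environment tool that scatters static meshes along a spline.
; Its construction script adds a mesh component at fixed distance intervals along the spline, with shared scale and randomized pitch and yaw.
; A seeded random stream drives both rotation and a pick from an array, which a switch maps to one of six mesh variables.
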(fn ConstructionScript
  (bind _randomize (Variables|Components|GetRandomize))
  (bind _returnvalue (Math|Random|RandomFloatinRangefromStream -5e+01 1e+02 _randomize))
  (for _index (range 0 (.ReturnValue (Math|Float|Division(WholeandRemainder) (Spline|GetSplineLength (Variables|Default|GetSpline)) (Variables|Components|GetDistance))))
    (bind _returnvalue_2 (AddComponent|AddStaticMeshComponent false (Math|Transform|MakeTransform (Spline|GetLocationatDistanceAlongSpline (Variables|Default|GetSpline) (* _index (Variables|Components|GetDistance)) "Local") (Math|Rotator|MakeRotator 0.0 _returnvalue _returnvalue) (Math|Conversions|ToVector(Float) (Variables|Components|GetScale)))))
    (switch string (.OutItem (Utilities|Array|RandomFromStream (Variables|Components|GetTarget%20Array) _randomize))
      (:Default
        (Components|StaticMesh|SetStaticMesh _returnvalue_2 (Variables|Procedural_Mesh_Spline|GetMesh) :!label _label))
      (:Case_0
        (goto _label))
      (:Case_1
        (Components|StaticMesh|SetStaticMesh _returnvalue_2 (Variables|ProceduralMeshSpline|GetMesh01)))
      (:Case_2
        (Components|StaticMesh|SetStaticMesh _returnvalue_2 (Variables|ProceduralMeshSpline|GetMesh02)))
      (:Case_3
        (Components|StaticMesh|SetStaticMesh _returnvalue_2 (Variables|ProceduralMeshSpline|GetMesh03)))
      (:Case_4
        (Components|StaticMesh|SetStaticMesh _returnvalue_2 (Variables|ProceduralMeshSpline|GetMesh04)))
      (:Case_5
        (Components|StaticMesh|SetStaticMesh _returnvalue_2 (Variables|ProceduralMeshSpline|GetMesh05) :!label _label_2))
      (:Case_6
        (goto _label_2)))))